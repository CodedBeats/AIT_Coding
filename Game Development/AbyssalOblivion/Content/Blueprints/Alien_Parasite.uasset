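; Alien parasite enemy built from three ring meshes that takes damage and freezes when killed.
; While alive, Tick calls SpinMeshes, where a looping MultiGate rotates one ring per frame in turn, each in its own direction.
; AnyDamage reduces Health; at zero it sets IsDead, which halts the spin, applies the frozen material to all rings and destroys the actor after a short delay.
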(event Custom|StopAnimation
  ;[0.2135 0.7584 1] Stop Animating Alien
  (Utilities|FlowControl|MultiGate false true -1
    (:Out%200
      (Transformation|AddLocalRotation (Variables|Default|Getring1) "0.000000,0.000000,0.000000" false false))
    (:Out%201
      (Transformation|AddLocalRotation (Variables|Default|Getring3) "0.000000,0.000000,0.000000" false false))
    (:Out%202
      (Transformation|AddLocalRotation (Variables|Default|Getring2) "0.000000,0.000000,0.000000" false false))))

(event Custom|Freeze
  ;[1 0.474 0.9347] Freeze
  (Rendering|Material|SetMaterial (Variables|Default|Getring1) 0 "/Game/Materials/Frozen_Alien.Frozen_Alien")
  (Rendering|Material|SetMaterial (Variables|Default|Getring2) 0 "/Game/Materials/Frozen_Alien.Frozen_Alien")
  (Rendering|Material|SetMaterial (Variables|Default|Getring3) 0 "/Game/Materials/Frozen_Alien.Frozen_Alien")
  (CallFunction|StopAnimation))

(event Custom|SpinMeshes
  ;[0.2135 0.7584 1] Animate Alien
  (Utilities|FlowControl|MultiGate false true -1
    (:Out%200
      (Transformation|AddLocalRotation (Variables|Default|Getring1) "0.000000,0.000000,20.000000" false false))
    (:Out%201
      (Transformation|AddLocalRotation (Variables|Default|Getring3) "0.000000,0.000000,-20.000000" false false))
    (:Out%202
      (Transformation|AddLocalRotation (Variables|Default|Getring2) "20.000000,0.000000,0.000000" false false))))

(event EventTick
  (params (DeltaSeconds :type Float%20%28single-precision%29))
  ;[1 0.5765 0.1602] Init
  (if (not (Variables|Default|GetisDead))
    (CallFunction|SpinMeshes)))

(event Game|Damage|EventAnyDamage
  (params (Damage :type Float%20%28single-precision%29) (DamageType :type Damage%20Type%20Object%20Reference) (InstigatedBy :type Controller%20Object%20Reference) (DamageCauser :type Actor%20Object%20Reference))
  ;[1 0.3229 0.3229] Take Damage
  (if (not (Variables|Default|GetisDead))
    (Variables|Default|SetHealth (- (Variables|Default|GetHealth) Damage))
    (if (<= (Variables|Default|GetHealth) 0.0)
      (Variables|Default|SetisDead true)
      (CallFunction|Freeze)
      (Utilities|FlowControl|Delay 3.0)
      (Actor|DestroyActor))))

(fn ConstructionScript)