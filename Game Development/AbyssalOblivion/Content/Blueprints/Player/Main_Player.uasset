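; Player character for a zero-gravity space game who uses a fire extinguisher as both thruster and weapon against aliens.
; Enhanced Input drives LaunchCharacter bursts and propulsion along the camera axis, spending shared fuel/ammo that alien deaths refill.
; Backward thrust sprays goo forward and toggles a collision box that damages aliens.
; It also runs the HUD, timed tutorial, health, out-of-fuel screen, and death, notifying trackers and aliens.
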(event OnComponentBeginOverlap(FrontCollisionBox)
  (params (OverlappedComponent :type Primitive%20Component%20Object%20Reference) (OtherActor :type Actor%20Object%20Reference) (OtherComp :type Primitive%20Component%20Object%20Reference) (OtherBodyIndex :type Integer) (bFromSweep :type Boolean) (SweepResult :type Hit%20Result%20Structure%20%28by%20ref%29))
  ;[1 0.9228 0.2969] Check Collision with Alien
  (if (Components|ComponentHasTag OtherComp "AlienCollisionBox")
    (CallFunction|UpdateUICrosshair (Variables|Default|GetcrosshairHit))
    (Collision|SetCollisionEnabled (Variables|Default|GetFrontCollisionBox) "NoCollision") ; disable collision to refresh
    (Utilities|FlowControl|Delay 0.1)
    (Game|Damage|ApplyDamage OtherActor 2.0 0 0)
    (Audio|PlaySoundatLocation "/Game/Audio/Alien/get_hit_by_player.get_hit_by_player" "0, 0, 0" "0, 0, 0" 1.0 1.0 0.0 0 0 0 0)
    (CallFunction|UpdateUICrosshair (Variables|Default|GetcrosshairDefault))))

(event Custom|PropelBackward
  ;[0.08627 0.3569 0.8745] Move Backward
  ;;[0.08627 0.3569 0.8745] Propel
  (if (not (Variables|Default|GetisBursting))
    (Variables|Default|Setspeed 0.3)
    (bind _output_get (Variables|Default|SetmovementDirection (Math|Vector|GetForwardVector (Variables|Default|GetCamera))))
    (Character|LaunchCharacter (* _output_get (Variables|Default|Getspeed) -1) false false)))

(event Custom|ToggleOnCollision
  ;[1 0.9228 0.2969] Toggle Collision Box
  (if (Variables|Default|GetisShooting)
    (Collision|SetCollisionEnabled (Variables|Default|GetFrontCollisionBox) "QueryAndPhysics")
    (else
      (Collision|SetCollisionEnabled (Variables|Default|GetFrontCollisionBox) "NoCollision"))))

(event Custom|TriggerBpEvents
  ;[1 0.2014 0.6084] Trigger Blueprint Events on Player Death
  (bind _outactors (Actor|GetAllActorswithInterface "/Game/Blueprints/Player/PlayerDeath_Interface.PlayerDeath_Interface_C"))
  (for _array_element _outactors
    (bind _astracker (Utilities|Casting|CastToTracker _array_element)
      (:then
        (Class|PlayerDeathInterface|OnPlayerDeath(Message) _astracker))
      (:CastFailed
        (bind _asalien_parasite (Utilities|Casting|CastToAlien_Parasite _array_element))
        (Class|PlayerDeathInterface|OnPlayerDeath(Message) _asalien_parasite)))))

(event Custom|RefillAmmo
  (params (refilAmount :type Float%20%28double-precision%29))
  ;[0.2454 0.9203 1] Refill Ammo
  (Audio|PlaySoundatLocation "/Game/Interface_And_Item_Sounds/WAV/Item_Sell_Purchase_05.Item_Sell_Purchase_05" "0, 0, 0" "0, 0, 0" 1.0 1.0 0.0 0 0 0 0)
  (Variables|Default|Setammo (+ (Variables|Default|Getammo) refilAmount))
  (if (> (Variables|Default|Getammo) (Variables|Default|GetmaxAmmo))
    (Variables|Default|SetmaxAmmo (Variables|Default|Getammo))))

(event Custom|PlayGetHitSound
  ;[0.3569 1 0.4039] Get Hit by Alien Sound
  (Utilities|FlowControl|DoOnce false :!label _label
    (:Completed
      (Audio|PlaySoundatLocation "/Game/Audio/Player/get_hit_by_alien.get_hit_by_alien" (Transformation|GetWorldLocation (Variables|Default|GetCamera)) "0, 0, 0" 1.0 1.0 0.0 0 0 0 0)
      (Utilities|FlowControl|Delay 1.0)
      (goto _label Reset))))

(event Custom|SetPlayerAdrift
  ;[0.371 0.1232 1] Set Player Adrift if they run out of fuel
  (if (== (Variables|Default|Getammo) 0.0)
    (Utilities|FlowControl|DoOnce false
      (:Completed
        (Viewport|RemoveAllWidgets)
        (bind _returnvalue (UserInterface|CreateWidget "/Game/UI/MainGame_UI/NoFuel_UI.NoFuel_UI_C"))
        (UserInterface|Viewport|AddtoViewport _returnvalue 0)))))

(event Custom|SetupTutorial
  ;[0.3725 0.1216 1] Tutorial UI
  ;;[0.3725 0.1216 1] Pickup Fire Extingusher
  (bind _returnvalue (UserInterface|CreateWidget "/Game/UI/Tutorial.Tutorial_C"))
  (bind _output_get (Variables|Default|SettutorialUI _returnvalue))
  (UserInterface|Viewport|AddtoViewport _output_get 0)
  (Variables|Default|SetinTutorial true)
  (Default|AddText (Variables|Default|GettutorialUI) (Utilities|Text|FormatText "Tutorial - (\"T\" to skip)") (Utilities|Text|FormatText "Pickup the Fire Extinguisher 
You cannot move in a vaccum")))

(event Custom|AquireExtinguisher
  ;[1 0.2014 0.6084] Pickup Fire Extinguisher
  (Variables|Default|SetcanMove true) ; Allow movement
  (Rendering|SetVisibility (Variables|Default|Getflamethrower02) true false) ; Show Weapon
  (Variables|Default|Setammo 3.5e+02) ; Add Base Ammo
  (CallFunction|DisplayTutorialMessages))

(event Custom|ExplainWeaponMovementTutorial
  ;[0.3725 0.1216 1] Tutorial UI
  ;;[0.3725 0.1216 1] Explain Fire Extinguisher Movement
  (Default|AddText (Variables|Default|GettutorialUI) (Utilities|Text|FormatText "Forward Propulsion 
Tap Left Click - Burst Propulsion 
Hold Left Click - Medium Propulsion") (Utilities|Text|FormatText "Tapping left click consumes more fuel but helps speed you up 
Holding left click consumes less fuel but is bad at slowing you down")))

(event Custom|ExplainWeaponShootungTutorial
  ;[0.3725 0.1216 1] Tutorial UI
  ;;[0.3725 0.1216 1] Explain Fire Extinguisher Shooting
  (Default|AddText (Variables|Default|GettutorialUI) (Utilities|Text|FormatText "Shooting/Backward Propulsion 
Hold Right Click - Shoot Forward") (Utilities|Text|FormatText "Shoot forward to help target and freeze enemies 
This will move you backwards as well but very slowly 
Freezing an enemy will give you some fuel back")))

(event Custom|ExplainMagnetBootsTutorial
  ;[0.3725 0.1216 1] Tutorial UI
  ;;[0.3725 0.1216 1] Explain Magnet Boots (its not a bug, it's a feature lol)
  (Default|AddText (Variables|Default|GettutorialUI) (Utilities|Text|FormatText "Magent Boots") (Utilities|Text|FormatText "You have Magent Boots on, if your feet touch the space station you stick 
You can easily detach just by using the fire extinguisher movement")))

(event Custom|DisplayTutorialMessages
  ;[0.3725 0.1216 1] Tutorial UI
  ;;[0.3725 0.1216 1] Display All Tutorial Messages
  (CallFunction|ExplainWeaponMovementTutorial)
  (Utilities|FlowControl|Delay 15.0)
  (CallFunction|ExplainWeaponShootungTutorial)
  (Utilities|FlowControl|Delay 15.0)
  (CallFunction|ExplainHP&FuelTutorial)
  (Utilities|FlowControl|Delay 15.0)
  (CallFunction|ExplainPickupsTutorial)
  (Utilities|FlowControl|Delay 15.0)
  (CallFunction|ExplainMagnetBootsTutorial)
  (Utilities|FlowControl|Delay 15.0)
  (Widget|RemovefromParent (Variables|Default|GettutorialUI))
  (Variables|Default|SetinTutorial false))

(event Custom|ShootWhiteGoo
  (bind _forwardnozzlearrow (Variables|Default|GetforwardNozzleArrow))
  (bind _backwardnozzlearrow (Variables|Default|GetbackwardNozzleArrow))
  ;[1 0.4863 0.4863] Shoot
  (if (Variables|Default|GetisShooting)
    (if (> (Variables|Default|Getammo) 0.0)
      (if (Variables|Default|GetisPropelledBackward)
        (Niagara|SpawnSystematLocation "/Game/VFX/Extringuihser_Goo.Extringuihser_Goo" (Transformation|GetWorldLocation _forwardnozzlearrow) (Transformation|GetWorldRotation _forwardnozzlearrow) (Transformation|GetWorldScale _forwardnozzlearrow))
        (CallFunction|PlayFireForwardSound)
        (Utilities|FlowControl|Delay 0.2)
        (Math|Float|DecrementFloat (Variables|Default|Getammo)
          (:%20%20
            (CallFunction|SetPlayerAdrift)))
        (elif (Variables|Default|GetisPropelledForward)
          (Niagara|SpawnSystematLocation "/Game/VFX/Extringuihser_Goo.Extringuihser_Goo" (Transformation|GetWorldLocation _backwardnozzlearrow) (Transformation|GetWorldRotation _backwardnozzlearrow) (Transformation|GetWorldScale _backwardnozzlearrow))
          (CallFunction|PlayFireBackSound)
          (Utilities|FlowControl|Delay 0.1)
          (Math|Float|DecrementFloat (Variables|Default|Getammo)
            (:%20%20
              (CallFunction|SetPlayerAdrift)))))
      (else
        (Variables|Default|SetcanShoot false)))))

(event Custom|ExplainPickupsTutorial
  ;[0.3725 0.1216 1] Tutorial UI
  ;;[0.3725 0.1216 1] Explain Pickups
  (Default|AddText (Variables|Default|GettutorialUI) (Utilities|Text|FormatText "Pickups") (Utilities|Text|FormatText "The spinning Fire Extinguisher and Health Pack are pickups 
Regain some health or fuel by moving through them 
You can exceed your max ammo but not your max health")))

(event Custom|ExplainHP&FuelTutorial
  ;[0.3725 0.1216 1] Tutorial UI
  ;;[0.3725 0.1216 1] Explain Health and Ammo
  (Default|AddText (Variables|Default|GettutorialUI) (Utilities|Text|FormatText "Health & Fuel") (Utilities|Text|FormatText "If you hit 0 Health you will die 
If you run out of fuel you will drift in space forever 
(In both these cases you will be able to respawn from the start)")))

(event Custom|SkipTutorial
  ;[0.3725 0.1216 1] Tutorial UI
  ;;[0.3725 0.1216 1] Skip Tutorial
  (if (Variables|Default|GetinTutorial)
    (Widget|RemovefromParent (Variables|Default|GettutorialUI))))

(event Custom|Die
  ;[1 0.4863 0.4863] Die
  (Viewport|RemoveAllWidgets)
  (bind _returnvalue (UserInterface|CreateWidget "/Game/UI/MainGame_UI/Death_UI.Death_UI_C"))
  (UserInterface|Viewport|AddtoViewport _returnvalue 0)
  (CallFunction|TriggerBpEvents)
  (Actor|DestroyActor))

(event Custom|RefillHealth
  (params (refilAmount :type Float%20%28double-precision%29))
  ;[0.2454 0.9203 1] Refill Health
  (Variables|Default|Sethealth (Math|Float|Clamp(Float) (+ (Variables|Default|Gethealth) refilAmount) 0.0 (Variables|Default|GetmaxHealth)))
  (Audio|PlaySoundatLocation "/Game/Audio/UI/health_pickup.health_pickup" "0, 0, 0" "0, 0, 0" 1.0 1.0 0.0 0 0 0 0))

(event Custom|PlayFireForwardSound
  ;[0.3569 1 0.4039] Firing Sound
  ;;[0.3569 1 0.4039] Fire Forward
  (Utilities|FlowControl|DoOnce false :!label _label
    (:Completed
      (Audio|PlaySoundatLocation "/Game/Audio/Weapon/fire_extinguisher_spray2.fire_extinguisher_spray2" (Transformation|GetWorldLocation (Variables|Default|GetforwardNozzleArrow)) "0, 0, 0" 1.0 1.0 0.0 0 0 0 0)
      (Utilities|FlowControl|Delay 0.35)
      (goto _label Reset))))

(event Custom|PropelForward
  ;[0.08627 0.3569 0.8745] Move Forward
  ;;[0.08627 0.3569 0.8745] Propel
  (if (not (Variables|Default|GetisBursting))
    (bind _output_get (Variables|Default|SetmovementDirection (Math|Vector|GetForwardVector (Variables|Default|GetCamera))))
    (Variables|Default|Setspeed 2.5)
    (Character|LaunchCharacter (* _output_get (Variables|Default|Getspeed)) false false)))

(event Custom|Burst
  ;[0.08627 0.3569 0.8745] Move Forward
  ;;[0.08627 0.3569 0.8745] Small Burst
  (if (not (Variables|Default|GetisBursting))
    (bind _output_get (Variables|Default|SetmovementDirection (Math|Vector|GetForwardVector (Variables|Default|GetCamera))))
    (Variables|Default|Setspeed 5e+02)
    (Character|LaunchCharacter (* _output_get (Variables|Default|Getspeed)) false false)
    (Variables|Default|Setammo (Math|Float|Clamp(Float) (- (Variables|Default|Getammo) 1e+01) 0.0 (Variables|Default|GetmaxAmmo))) ; Burst takes more ammo
    (CallFunction|SetPlayerAdrift)))

(event Custom|UpdateUICrosshair
  (params (crosshairImg :type Texture%20Object%20Reference))
  ;[0.371 0.1232 1] Toggle Crosshair
  (bind _output_get (Variables|Default|Setcrosshair crosshairImg))
  (Default|UpdateCrosshair (Variables|Default|GetHUD) _output_get))

(event Custom|PlayFireBackSound
  ;[0.3569 1 0.4039] Firing Sound
  ;;[0.3569 1 0.4039] Fire Backward
  (Utilities|FlowControl|DoOnce false :!label _label
    (:Completed
      (Audio|PlaySoundatLocation "/Game/Audio/Weapon/fire_extinguisher_spray2.fire_extinguisher_spray2" (Transformation|GetWorldLocation (Variables|Default|GetbackwardNozzleArrow)) "0, 0, 0" 1.0 1.0 0.0 0 0 0 0)
      (Utilities|FlowControl|Delay 0.35)
      (goto _label Reset))))

(event Input|EnhancedActionEvents|EnhancedInputActionSkip_Tutorial
  (params (ActionValue :type Boolean) (ElapsedSeconds :type Float%20%28double-precision%29) (TriggeredSeconds :type Float%20%28double-precision%29) (InputAction :type Input%20Action%20Object%20Reference :default "/Game/Core/InputActions/Skip_Tutorial.Skip_Tutorial"))
  ;[0.3725 0.1216 1] Tutorial UI
  ;;[0.3725 0.1216 1] Skip Tutorial
  (CallFunction|SkipTutorial))

(event Input|EnhancedActionEvents|EnhancedInputActionMouseMovement
  (params (ActionValue :type Vector%202D%20Structure) (ElapsedSeconds :type Float%20%28double-precision%29) (TriggeredSeconds :type Float%20%28double-precision%29) (InputAction :type Input%20Action%20Object%20Reference :default "/Game/Core/InputActions/MouseMovement.MouseMovement"))
  ;[0.08627 0.3569 0.8745] Mouse Movement
  (Pawn|Input|AddControllerYawInput (* (.x ActionValue) 0.7)) ; Turn Left and Right
  (Pawn|Input|AddControllerPitchInput (* (* (.y ActionValue) 0.7) -1.0)) ; Turns Up and Down
)

(event Input|EnhancedActionEvents|EnhancedInputActionExtinguish_Fire
  (params (ActionValue :type Boolean) (ElapsedSeconds :type Float%20%28double-precision%29) (TriggeredSeconds :type Float%20%28double-precision%29) (InputAction :type Input%20Action%20Object%20Reference :default "/Game/Core/InputActions/Extinguish_Fire.Extinguish_Fire"))
  ;[0.08627 0.3569 0.8745] Move Backward
  ;;[0.08627 0.3569 0.8745] Conditions
  (:Triggered
    (if (Variables|Default|GetcanMove)
      (if (Variables|Default|GetcanShoot)
        (Variables|Default|SetisShooting true)
        (Variables|Default|SetisPropelledBackward true)
        (CallFunction|PropelBackward)
        (CallFunction|ShootWhiteGoo)
        (CallFunction|ToggleonCollision))))
  (:Completed
    (Variables|Default|SetisShooting false)
    (Variables|Default|SetisPropelledBackward false)))

(event Input|EnhancedActionEvents|EnhancedInputActionExtinguish_Move
  (params (ActionValue :type Boolean) (ElapsedSeconds :type Float%20%28double-precision%29) (TriggeredSeconds :type Float%20%28double-precision%29) (InputAction :type Input%20Action%20Object%20Reference :default "/Game/Core/InputActions/Extinguish_Move.Extinguish_Move"))
  ;[0.08627 0.3569 0.8745] Move Forward
  ;;[0.08627 0.3569 0.8745] Conditions
  (:Triggered
    (if (Variables|Default|GetcanMove)
      (Variables|Default|SetisShooting true)
      (Variables|Default|SetisPropelledForward true)
      (CallFunction|PropelForward)
      (CallFunction|ShootWhiteGoo)))
  (:Started
    (if (Variables|Default|GetcanMove)
      (if (Variables|Default|GetcanShoot)
        (Variables|Default|SetisShooting true)
        (Variables|Default|SetisPropelledForward true)
        (CallFunction|Burst)
        (Variables|Default|SetisBursting true)
        (CallFunction|ShootWhiteGoo)
        (Utilities|FlowControl|Delay 0.2)
        (Variables|Default|SetisBursting false))))
  (:Canceled
    (Variables|Default|SetisShooting false)
    (Variables|Default|SetisPropelledForward false)))

(event EventBeginPlay
  ;[1 0.4232 0.125] Init
  (Input|AddMappingContext (PlayerController|LocalPlayerSubsystems|GetEnhancedInputLocalPlayerSubsystem (Game|GetPlayerController 0)) "/Game/Core/AO_Main_IMC.AO_Main_IMC" 0 "(bIgnoreAllPressedKeysUntilRelease=True,bForceImmediately=False,bNotifyUserSettings=False)") ; Select the IMC to use
  (bind _returnvalue (UserInterface|CreateWidget "/Game/UI/MainGame_UI/HUD.HUD_C"))
  (bind _output_get (Variables|Default|SetHUD _returnvalue))
  (UserInterface|Viewport|AddtoViewport _output_get 0)
  (CallFunction|SetupTutorial))

(event Game|Damage|EventAnyDamage
  (params (Damage :type Float%20%28single-precision%29) (DamageType :type Damage%20Type%20Object%20Reference) (InstigatedBy :type Controller%20Object%20Reference) (DamageCauser :type Actor%20Object%20Reference))
  ;[1 0.4863 0.4863] Loose Health
  (if (> (Variables|Default|Gethealth) 0.0)
    (Variables|Default|SetHealth (Math|Float|Clamp(Float) (- (Variables|Default|GetHealth) Damage) 0.0 (Variables|Default|GetmaxHealth)))
    (CallFunction|PlayGetHitSound)
    (else
      (CallFunction|Die))))

(event EventOnAlienDeath
  ;[1 0.4863 0.4863] Refill Some Ammo on Alien Death
  (CallFunction|RefillAmmo 5e+01))

(fn ConstructionScript)