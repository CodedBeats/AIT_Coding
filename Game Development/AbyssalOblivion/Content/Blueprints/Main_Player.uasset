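; Player character that uses a fire extinguisher both to move and to attack Alien_Parasite enemies, with mouse look through Enhanced Input.
; Extinguish_Fire nudges the player against the camera direction, sprays from the forward nozzle and enables a front collision box that deals delayed damage on overlap.
; Extinguish_Move starts with a forward burst, then sustains gentler forward thrust with spray from the backward nozzle.
; LaunchCharacter drives all propulsion, with a short IsBursting lock preventing stacked launches.
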(event OnComponentBeginOverlap(FrontCollisionBox)
  (params (OverlappedComponent :type Primitive%20Component%20Object%20Reference) (OtherActor :type Actor%20Object%20Reference) (OtherComp :type Primitive%20Component%20Object%20Reference) (OtherBodyIndex :type Integer) (bFromSweep :type Boolean) (SweepResult :type Hit%20Result%20Structure%20%28by%20ref%29))
  ;[1 0.9228 0.2969] Check Collision with Alien
  (bind _asalien_parasite (Utilities|Casting|CastToAlien_Parasite OtherActor)) ; can only collide with alien
  (Collision|SetCollisionEnabled (Variables|Default|GetFrontCollisionBox) "NoCollision") ; disable collision to refresh
  (Utilities|FlowControl|Delay 0.2)
  (Game|Damage|ApplyDamage _asalien_parasite 5.0 0 0))

(event Custom|PropelBackward
  ;[0.08627 0.3569 0.8745] Move Backward
  ;;[0.08627 0.3569 0.8745] Propel
  (if (not (Variables|Default|GetisBursting))
    (Variables|Default|Setspeed 0.3)
    (bind _output_get (Variables|Default|SetmovementDirection (Math|Vector|GetForwardVector (Variables|Default|GetCamera))))
    (Character|LaunchCharacter (* _output_get (Variables|Default|Getspeed) -1) false false)))

(event Custom|ToggleOnCollision
  ;[1 0.9228 0.2969] Toggle Collision Box
  (if (Variables|Default|GetisShooting)
    (Collision|SetCollisionEnabled (Variables|Default|GetFrontCollisionBox) "QueryAndPhysics")
    (else
      (Collision|SetCollisionEnabled (Variables|Default|GetFrontCollisionBox) "NoCollision"))))

(event Custom|ShootWhiteGoo
  (bind _forwardnozzlearrow (Variables|Default|GetforwardNozzleArrow))
  (bind _backwardnozzlearrow (Variables|Default|GetbackwardNozzleArrow))
  ;[1 0.4844 0.4844] Shoot
  (if (Variables|Default|GetisShooting)
    (if (Variables|Default|GetisPropelledBackward)
      (Niagara|SpawnSystematLocation "/Game/VFX/Extringuihser_Goo.Extringuihser_Goo" (Transformation|GetWorldLocation _forwardnozzlearrow) (Transformation|GetWorldRotation _forwardnozzlearrow) (Transformation|GetWorldScale _forwardnozzlearrow))
      (Audio|PlaySoundatLocation 0 (Transformation|GetWorldLocation (Variables|Default|GetforwardNozzleArrow)) "0, 0, 0" 1.0 1.0 0.0 0 0 0 0)
      (elif (Variables|Default|GetisPropelledForward)
        (Niagara|SpawnSystematLocation "/Game/VFX/Extringuihser_Goo.Extringuihser_Goo" (Transformation|GetWorldLocation _backwardnozzlearrow) (Transformation|GetWorldRotation _backwardnozzlearrow) (Transformation|GetWorldScale _backwardnozzlearrow))
        (Audio|PlaySoundatLocation 0 (Transformation|GetWorldLocation (Variables|Default|GetbackwardNozzleArrow)) "0, 0, 0" 1.0 1.0 0.0 0 0 0 0)))))

(event Custom|PropelForward
  ;[0.08627 0.3569 0.8745] Move Forward
  ;;[0.08627 0.3569 0.8745] Propel
  (if (not (Variables|Default|GetisBursting))
    (bind _output_get (Variables|Default|SetmovementDirection (Math|Vector|GetForwardVector (Variables|Default|GetCamera))))
    (Variables|Default|Setspeed 2.5)
    (Character|LaunchCharacter (* _output_get (Variables|Default|Getspeed)) false false)))

(event Custom|Burst
  ;[0.08627 0.3569 0.8745] Move Forward
  ;;[0.08627 0.3569 0.8745] Small Burst
  (if (not (Variables|Default|GetisBursting))
    (bind _output_get (Variables|Default|SetmovementDirection (Math|Vector|GetForwardVector (Variables|Default|GetCamera))))
    (Variables|Default|Setspeed 5e+02)
    (Character|LaunchCharacter (* _output_get (Variables|Default|Getspeed)) false false)))

(event Input|EnhancedActionEvents|EnhancedInputActionMouseMovement
  (params (ActionValue :type Vector%202D%20Structure) (ElapsedSeconds :type Float%20%28double-precision%29) (TriggeredSeconds :type Float%20%28double-precision%29) (InputAction :type Input%20Action%20Object%20Reference :default "/Game/Core/MouseMovement.MouseMovement"))
  ;[0.08627 0.3569 0.8745] Mouse Movement
  (Pawn|Input|AddControllerYawInput (.x ActionValue)) ; Turn Left and Right
  (Pawn|Input|AddControllerPitchInput (* (.y ActionValue) -1.0)) ; Turns Up and Down
)

(event Input|EnhancedActionEvents|EnhancedInputActionExtinguish_Fire
  (params (ActionValue :type Boolean) (ElapsedSeconds :type Float%20%28double-precision%29) (TriggeredSeconds :type Float%20%28double-precision%29) (InputAction :type Input%20Action%20Object%20Reference :default "/Game/Core/Extinguish_Fire.Extinguish_Fire"))
  ;[0.08627 0.3569 0.8745] Move Backward
  ;;[0.08627 0.3569 0.8745] Conditions
  (:Triggered
    (Variables|Default|SetisShooting true)
    (Variables|Default|SetisPropelledBackward true)
    (CallFunction|PropelBackward)
    (CallFunction|ShootWhiteGoo)
    (CallFunction|ToggleonCollision))
  (:Completed
    (Variables|Default|SetisShooting false)
    (Variables|Default|SetisPropelledBackward false)))

(event Input|EnhancedActionEvents|EnhancedInputActionExtinguish_Move
  (params (ActionValue :type Boolean) (ElapsedSeconds :type Float%20%28double-precision%29) (TriggeredSeconds :type Float%20%28double-precision%29) (InputAction :type Input%20Action%20Object%20Reference :default "/Game/Core/Extinguish_Move.Extinguish_Move"))
  ;[0.08627 0.3569 0.8745] Move Forward
  ;;[0.08627 0.3569 0.8745] Conditions
  (:Triggered
    (Variables|Default|SetisShooting true)
    (Variables|Default|SetisPropelledForward true)
    (CallFunction|PropelForward)
    (CallFunction|ShootWhiteGoo))
  (:Started
    (Variables|Default|SetisShooting true)
    (Variables|Default|SetisPropelledForward true)
    (CallFunction|Burst)
    (Variables|Default|SetisBursting true)
    (CallFunction|ShootWhiteGoo)
    (Utilities|FlowControl|Delay 0.2)
    (Variables|Default|SetisBursting false))
  (:Canceled
    (Variables|Default|SetisShooting false)
    (Variables|Default|SetisPropelledForward false)))

(event EventBeginPlay
  ;[1 0.4232 0.125] Init
  (Input|AddMappingContext (PlayerController|LocalPlayerSubsystems|GetEnhancedInputLocalPlayerSubsystem (Game|GetPlayerController 0)) "/Game/Core/AO_Main_IMC.AO_Main_IMC" 0 "(bIgnoreAllPressedKeysUntilRelease=True,bForceImmediately=False,bNotifyUserSettings=False)") ; Select the IMC to use
)

(fn ConstructionScript)