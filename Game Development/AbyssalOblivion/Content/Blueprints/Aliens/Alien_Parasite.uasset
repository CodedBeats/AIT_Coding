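; Alien Parasite enemy character that spins its three rings, faces the player and hunts on sight.
; Pawn sensing launches it opposite the player camera's forward vector, rather than pathfinding, then halts it after a short drift.
; Its sphere overlap with the player's tagged collision box triggers a lightning attack and damage.
; Hits flash ice particles; at zero health it freezes, then bursts after a delay, notifies the player and destroys itself.
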(event OnComponentBeginOverlap(Sphere)
  (params (OverlappedComponent :type Primitive%20Component%20Object%20Reference) (OtherActor :type Actor%20Object%20Reference) (OtherComp :type Primitive%20Component%20Object%20Reference) (OtherBodyIndex :type Integer) (bFromSweep :type Boolean) (SweepResult :type Hit%20Result%20Structure%20%28by%20ref%29))
  ;[1 0.3216 0.3216] Attack Player
  (if (Components|ComponentHasTag OtherComp "PlayerCollisionBox")
    (Collision|SetCollisionEnabled (Variables|Default|GetSphere) "NoCollision") ; disable collision to refresh
    (if (not (Variables|Default|GetisDead))
      (Components|Activation|SetActive (Variables|Default|GetP_DOT_Lightning_01) true false) ; show electric attack
      (CallFunction|StopMovement)
      (Utilities|FlowControl|Delay 0.1)
      (Game|Damage|ApplyDamage OtherActor 1.0 0 0)
      (Collision|SetCollisionEnabled (Variables|Default|GetSphere) "QueryAndPhysics")
      (Utilities|FlowControl|Delay 0.5)
      (Components|Activation|SetActive (Variables|Default|GetP_DOT_Lightning_01) false false) ; hide electric attack
    )))

(event OnSeePawn(PawnSensing)
  (params (Pawn :type Pawn%20Object%20Reference))
  ;[0.3333 0.8902 1] Follow Player
  (bind _asmain_player (Utilities|Casting|CastToMain_Player Pawn))
  (if (not (Variables|Default|GetisDead))
    (Pawn|Components|CharacterMovement|SetMovementMode (Variables|Character|GetCharacterMovement) "MOVE_Walking" 0) ; allow movement
    (Character|LaunchCharacter (* (Math|Vector|GetForwardVector (Variables|/Game/Blueprints/Player/Main_Player.Main_Player_C|GetCamera _asmain_player)) -8.5e+02) false false) ; follow player
    (CallFunction|PlayHuntingSound)
    (Utilities|FlowControl|Delay 2.0) ; allow movement/drift for 2s
    (if (not (Variables|Default|GetisDead))
      (CallFunction|StopMovement) ; stop all movement
    )))

(event Custom|StopAnimation
  ;[1 0.4745 0.9333] Stop Animating Alien
  (Utilities|FlowControl|MultiGate false true -1
    (:Out%200
      (Transformation|AddLocalRotation (Variables|Default|Getring1) "0, 0, 0" false false))
    (:Out%201
      (Transformation|AddLocalRotation (Variables|Default|Getring3) "0, 0, 0" false false))
    (:Out%202
      (Transformation|AddLocalRotation (Variables|Default|Getring2) "0, 0, 0" false false))))

(event Custom|Freeze
  ;[1 0.4745 0.9333] Freeze
  (Rendering|Material|SetMaterial (Variables|Default|Getring1) 0 "/Game/Materials/Alien/Frozen_Alien.Frozen_Alien")
  (Rendering|Material|SetMaterial (Variables|Default|Getring2) 0 "/Game/Materials/Alien/Frozen_Alien.Frozen_Alien")
  (Rendering|Material|SetMaterial (Variables|Default|Getring3) 0 "/Game/Materials/Alien/Frozen_Alien.Frozen_Alien")
  (CallFunction|StopAnimation)
  (Components|DestroyComponent (Variables|Default|GetPointLight)))

(event Custom|StopMovement
  ;[0.3333 0.8902 1] Stop Movement
  (Physics|SetPhysicsLinearVelocity (Variables|Character|GetMesh) "0, 0, 0" false "None") ; Remove velocity
  (Pawn|Components|CharacterMovement|SetMovementMode (Variables|Character|GetCharacterMovement) "MOVE_None" 0) ; Remove movement
)

(event Custom|PlayHuntingSound
  (bind _returnvalue (Math|Random|RandomIntegerinRange 0 2))
  ;[0.3569 1 0.4039] Random Move Sounds
  (Utilities|FlowControl|MultiGate true true -1
    (:Out%200
      (if (== _returnvalue 0)
        (Audio|PlaySoundatLocation "/Game/Audio/Alien/huting1.huting1" "0, 0, 0" "0, 0, 0" 1.0 1.0 0.0 0 0 0 0)))
    (:Out%201
      (if (== _returnvalue 1)
        (Audio|PlaySoundatLocation "/Game/Audio/Alien/huting2.huting2" "0, 0, 0" "0, 0, 0" 1.0 1.0 0.0 0 0 0 0)))
    (:Out%202
      (if (== _returnvalue 2)
        (Audio|PlaySoundatLocation "/Game/Audio/Alien/huting3.huting3" "0, 0, 0" "0, 0, 0" 1.0 1.0 0.0 0 0 0 0)))))

(event Custom|PlayGetHitSound
  ;[0.3569 1 0.4039] Get Hit by Player Sound
  (Utilities|FlowControl|DoOnce false :!label _label
    (:Completed
      (Audio|PlaySoundatLocation "/Game/Audio/Alien/get_hit_by_player.get_hit_by_player" (Transformation|GetWorldLocation (Variables|Character|GetMesh)) "0, 0, 0" 1.0 1.0 0.0 0 0 0 0)
      (Utilities|FlowControl|Delay 2.0)
      (goto _label Reset))))

(event Custom|Die
  ;[1 0.3216 0.3216] Die
  (Rendering|SetVisibility (Variables|Default|GetRings) false true)
  (Components|Activation|SetActive (Variables|Default|GetP_Ice_Freeze_Motion_death) true false)
  (Class|AlienDeathInterface|OnAlienDeath(Message) (Game|Player|GetPlayerPawn 0))
  (Audio|PlaySoundatLocation "/Game/Audio/Alien/explode.explode" "0, 0, 0" "0, 0, 0" 1.0 1.0 0.0 0 0 0 0)
  (Utilities|FlowControl|Delay 3.0)
  (Actor|DestroyActor))

(event Custom|SpinMeshes
  ;[1 0.4745 0.9333] Animate Alien
  (Utilities|FlowControl|MultiGate false true -1
    (:Out%200
      (Transformation|AddLocalRotation (Variables|Default|Getring1) "0.000000,0.000000,20.000000" false false))
    (:Out%201
      (Transformation|AddLocalRotation (Variables|Default|Getring3) "0.000000,0.000000,-20.000000" false false))
    (:Out%202
      (Transformation|AddLocalRotation (Variables|Default|Getring2) "20.000000,0.000000,0.000000" false false))))

(event Custom|LookAtPlayer
  ;[0.3333 0.8902 1] Look at Player
  (Transformation|SetActorRotation (Math|Rotator|FindLookatRotation (Transformation|GetActorLocation) (Transformation|GetActorLocation (Game|Player|GetPlayerPawn 0)))))

(event EventOnPlayerDeath
  ;[1 0.3646 0.3646] Instant Destroy on Player Death
  (Actor|DestroyActor))

(event EventTick
  (params (DeltaSeconds :type Float%20%28single-precision%29))
  ;[1 0.5765 0.1602] Init
  (if (not (Variables|Default|GetisDead))
    (CallFunction|SpinMeshes)
    (CallFunction|LookatPlayer)))

(event Game|Damage|EventAnyDamage
  (params (Damage :type Float%20%28single-precision%29) (DamageType :type Damage%20Type%20Object%20Reference) (InstigatedBy :type Controller%20Object%20Reference) (DamageCauser :type Actor%20Object%20Reference))
  ;[1 0.3216 0.3216] Take Damage
  (if (not (Variables|Default|GetisDead))
    (Variables|Default|SetHealth (- (Variables|Default|GetHealth) Damage))
    (if (<= (Variables|Default|GetHealth) 0.0)
      (Variables|Default|SetisDead true)
      (CallFunction|Freeze)
      (Utilities|FlowControl|Delay 5.0)
      (CallFunction|Die)
      (else
        (CallFunction|PlayGetHitSound)
        (Components|Activation|SetActive (Variables|Default|GetP_Ice_Freeze_Motion) true false) ; show ice damage
        (Utilities|FlowControl|Delay 0.5)
        (Components|Activation|SetActive (Variables|Default|GetP_Ice_Freeze_Motion) false false) ; hide ice damae
      ))))

(fn ConstructionScript)