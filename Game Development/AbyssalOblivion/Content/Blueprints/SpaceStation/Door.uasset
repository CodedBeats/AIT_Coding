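; Space station door Blueprint that the player opens with the Interact input while inside its sensing volume.
; Overlapping AutomaticSensing with either player class enables input on the door and shows a prompt billboard.
; Interact hides the billboard and plays the DoorOpen timeline, which slides the door mesh along its local Y.
; Leaving the volume disables input, hides the billboard and reverses the timeline to close the door.
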(event OnComponentBeginOverlap(AutomaticSensing)
  (params (OverlappedComponent :type Primitive%20Component%20Object%20Reference) (OtherActor :type Actor%20Object%20Reference) (OtherComp :type Primitive%20Component%20Object%20Reference) (OtherBodyIndex :type Integer) (bFromSweep :type Boolean) (SweepResult :type Hit%20Result%20Structure%20%28by%20ref%29))
  ;[1 1 1] Give Player Input Control For Door
  (Utilities|Casting|CastToInitial_Player OtherActor
    (:then
      _)
    (:CastFailed
      (Utilities|Casting|CastToMain_Player OtherActor)))
  (Input|EnableInput (Game|GetPlayerController 0))
  (Rendering|SetVisibility (Variables|Default|GetBillboard) true false))

(event OnComponentEndOverlap(AutomaticSensing)
  (params (OverlappedComponent :type Primitive%20Component%20Object%20Reference) (OtherActor :type Actor%20Object%20Reference) (OtherComp :type Primitive%20Component%20Object%20Reference) (OtherBodyIndex :type Integer))
  ;[1 1 1] Open and Close Door
  (Utilities|Casting|CastToInitial_Player OtherActor
    (:then
      _)
    (:CastFailed
      (Utilities|Casting|CastToMain_Player OtherActor)))
  (Input|DisableInput (Game|GetPlayerController 0))
  (Rendering|SetVisibility (Variables|Default|GetBillboard) false false)
  (bind _dooropen (Timeline|DoorOpen Reverse)
    (:Update
      (Transformation|SetRelativeLocation (Variables|Default|GetSM_Door_1_Merged) (Math|Vector|MakeVector -93.0 _dooropen 48.0) false false))))

(event Input|EnhancedActionEvents|EnhancedInputActionInteract
  (params (ActionValue :type Boolean) (ElapsedSeconds :type Float%20%28double-precision%29) (TriggeredSeconds :type Float%20%28double-precision%29) (InputAction :type Input%20Action%20Object%20Reference :default "/Game/Core/Interact.Interact"))
  ;[1 1 1] Open and Close Door
  (Rendering|SetVisibility (Variables|Default|GetBillboard) false false)
  (bind _dooropen (Timeline|DoorOpen Play)
    (:Update
      (Transformation|SetRelativeLocation (Variables|Default|GetSM_Door_1_Merged) (Math|Vector|MakeVector -93.0 _dooropen 48.0) false false))))

(fn ConstructionScript)