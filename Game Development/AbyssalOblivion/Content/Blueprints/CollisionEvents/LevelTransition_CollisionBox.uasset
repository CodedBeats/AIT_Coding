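; LevelTransition_CollisionBox is a one-shot trigger volume that starts a worm attack event and then shows a loading screen.
; On overlap by any actor, it disables its collision, then broadcasts camera shake and worm trigger messages to every actor implementing those interfaces.
; After a delay it adds the Loading widget to the viewport, without opening a level itself.
; A parallel sequence branch immediately stops an overlapping Initial_Player's movement.
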(event OnComponentBeginOverlap(CollisionBox)
  (params (OverlappedComponent :type Primitive%20Component%20Object%20Reference) (OtherActor :type Actor%20Object%20Reference) (OtherComp :type Primitive%20Component%20Object%20Reference) (OtherBodyIndex :type Integer) (bFromSweep :type Boolean) (SweepResult :type Hit%20Result%20Structure%20%28by%20ref%29))
  ;[1 1 1] Trigger Worm Attack Ship Event
  (Utilities|FlowControl|Sequence
    (:then_0
      (Collision|SetCollisionEnabled (Variables|Default|GetCollisionBox) "NoCollision") ; Disable Collision for re-trigger
      (CallFunction|TriggerCameraShake)
      (CallFunction|TriggerWorm)
      (Utilities|FlowControl|Delay 7.0)
      (bind _returnvalue (UserInterface|CreateWidget "/Game/UI/Loading.Loading_C"))
      (UserInterface|Viewport|AddtoViewport _returnvalue 0))
    (:then_1
      (bind _asinitial_player (Utilities|Casting|CastToInitial_Player OtherActor))
      (Default|StopMovement _asinitial_player))))

(event Custom|TriggerWorm
  ;[1 1 1] Trigger Worm Move
  (bind _outactors (Actor|GetAllActorswithInterface "/Game/Blueprints/CollisionEvents/WormTriggerInterface.WormTriggerInterface_C"))
  (for _array_element _outactors
    (Class|WormTriggerInterface|OnWormTrigger(Message) _array_element)))

(event Custom|TriggerCameraShake
  ;[1 1 1] Trigger Player Camera Shake
  (bind _outactors (Actor|GetAllActorswithInterface "/Game/Blueprints/Player/CameraShake_Interface.CameraShake_Interface_C"))
  (for _array_element _outactors
    (Class|CameraShakeInterface|OnCameraShake(Message) _array_element)))

(fn ConstructionScript)