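; Tracker actor that marks the escape capsule with a floating debug readout of the player's distance to it.
; Every tick it measures the 2D distance between itself and the player pawn.
; It draws that value as a debug string with a downward arrow at its DebugStringLocation component's world position.
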(event Custom|Track
  ;[0.2708 0.2708 0.2708] Show Distance to Target
  (bind _output_get (Variables|Default|SetdistanceToPlayer (Math|Vector|Distance2D(Vector) (Transformation|GetActorLocation) (Transformation|GetActorLocation (Game|Player|GetPlayerPawn 0)))))
  (Rendering|Debug|DrawDebugString (Transformation|GetWorldLocation (Variables|Default|GetDebugStringLocation)) (Utilities|String|ToString(Text) (Utilities|Text|FormatText "Escape Capsule: {distanceVal} 
                          ↓" _output_get)) 0 "(R=1.000000,G=1.000000,B=1.000000,A=1.000000)"))

(event EventTick
  (params (DeltaSeconds :type Float%20%28single-precision%29))
  ;[0.2708 0.2708 0.2708] Show Distance to Target
  (CallFunction|Track))

(fn ConstructionScript)